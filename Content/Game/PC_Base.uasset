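; Base player controller that sets up Enhanced Input and routes player input to the BP_Chara character.
; Handles look, yaw-relative movement and jump directly, while Rallonge, Roar and Dash are forwarded to the character.
; Pause and the Unpause event share a FlipFlop that toggles game pause and notifies HUD_Main.
; Grounded punches play a montage with movement disabled, restoring walking on montage completion or input release.
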(event `self.ReceiveBeginPlay`
  (bind _returnvalue (pcsubsystem `EnhancedInputLocalPlayerSubsystem` self))
  ;[1 1 1] Mapping
  (bind _returnvalue_2 (`GameplayStatics.GetActorOfClass` "/Game/BP/BP_Chara.BP_Chara_C"))
  (set `self.Player_ref` _returnvalue_2)
  (`/Engine/EditorBlueprintResources/StandardMacros.IsValid` _returnvalue
    (:`Is Valid`
      (`EnhancedInputSubsystemInterface.AddMappingContext` _returnvalue "/Game/Input/IMC_Player.IMC_Player" 0 (struct)))))

(event `EnhancedInput|/Game/Input/IA_Look`
  (params (ActionValue :type "Vector2D Structure") (ElapsedSeconds :type "Float (double-precision)") (TriggeredSeconds :type "Float (double-precision)") (InputAction :type "InputAction Object Reference" :default "/Game/Input/IA_Look.IA_Look"))
  ;[1 1 1] Camera
  (:`Triggered`
    (`self.AddYawInput` ActionValue_X)
    (`self.AddPitchInput` ActionValue_Y)))

(event `EnhancedInput|/Game/Input/IA_Pause`
  (params (ActionValue :type Boolean) (ElapsedSeconds :type "Float (double-precision)") (TriggeredSeconds :type "Float (double-precision)") (InputAction :type "InputAction Object Reference" :default "/Game/Input/IA_Pause.IA_Pause"))
  ;[1 1 1] Pause
  (:`Started`
    (`/Engine/EditorBlueprintResources/StandardMacros.FlipFlop` :!label _label
      (:`A`
        (`GameplayStatics.SetGamePaused` true))
      (:`B`
        (`GameplayStatics.SetGamePaused` false)))
    (bind _ashud_main (cast `/Game/Game/HUD_Main` (`self.GetHUD`)))
    (`/Game/Game/HUD_Main.Event UIpause` _ashud_main)))

(event `EnhancedInput|/Game/Input/IA_Move`
  (params (ActionValue :type "Vector2D Structure") (ElapsedSeconds :type "Float (double-precision)") (TriggeredSeconds :type "Float (double-precision)") (InputAction :type "InputAction Object Reference" :default "/Game/Input/IA_Move.IA_Move"))
  (bind (_returnvalue_roll _returnvalue_pitch _returnvalue_yaw) (`KismetMathLibrary.BreakRotator` (`self.GetControlRotation`)))
  (bind _player_ref (`self.Player_ref`))
  ;[1 1 1] Movement
  (:`Triggered`
    (`Pawn.AddMovementInput` _player_ref (`KismetMathLibrary.GetRightVector` (`KismetMathLibrary.MakeRotator` _returnvalue_roll 0.0 _returnvalue_yaw)) ActionValue_X false)
    (`Pawn.AddMovementInput` _player_ref (`KismetMathLibrary.GetForwardVector` (`KismetMathLibrary.MakeRotator` 0.0 0.0 _returnvalue_yaw)) ActionValue_Y false)))

(event `Unpause`
  ;[1 1 1] Pause
  (goto _label))

(event `EnhancedInput|/Game/Input/IA_Jump`
  (params (ActionValue :type Boolean) (ElapsedSeconds :type "Float (double-precision)") (TriggeredSeconds :type "Float (double-precision)") (InputAction :type "InputAction Object Reference" :default "/Game/Input/IA_Jump.IA_Jump"))
  (bind _returnvalue (`GameplayStatics.GetPlayerCharacter` 0))
  ;[1 1 1] Actions
  (:`Started`
    (`Character.Jump` _returnvalue))
  (:`Completed`
    (`Character.StopJumping` _returnvalue)))

(event `EnhancedInput|/Game/Input/IA_Rallonge`
  (params (ActionValue :type Boolean) (ElapsedSeconds :type "Float (double-precision)") (TriggeredSeconds :type "Float (double-precision)") (InputAction :type "InputAction Object Reference" :default "/Game/Input/IA_Rallonge.IA_Rallonge"))
  ;[1 1 1] Actions
  (:`Started`
    (bind _asbp_chara (cast `/Game/BP/BP_Chara` (`GameplayStatics.GetPlayerCharacter` 0)))
    (`/Game/BP/BP_Chara.Rallonge` _asbp_chara)))

(event `EnhancedInput|/Game/Input/IA_Roar`
  (params (ActionValue :type Boolean) (ElapsedSeconds :type "Float (double-precision)") (TriggeredSeconds :type "Float (double-precision)") (InputAction :type "InputAction Object Reference" :default "/Game/Input/IA_Roar.IA_Roar"))
  ;[1 1 1] Actions
  (:`Started`
    (bind _asbp_chara (cast `/Game/BP/BP_Chara` (`GameplayStatics.GetPlayerCharacter` 0)))
    (`/Game/BP/BP_Chara.Roared` _asbp_chara)))

(event `EnhancedInput|/Game/Input/IA_Dash`
  (params (ActionValue :type Boolean) (ElapsedSeconds :type "Float (double-precision)") (TriggeredSeconds :type "Float (double-precision)") (InputAction :type "InputAction Object Reference" :default "/Game/Input/IA_Dash.IA_Dash"))
  ;[1 1 1] Actions
  (:`Started`
    (bind _asbp_chara (cast `/Game/BP/BP_Chara` (`GameplayStatics.GetPlayerCharacter` 0)))
    (`/Game/BP/BP_Chara.Dash` _asbp_chara)))

(event `EnhancedInput|/Game/Input/IA_Punch`
  (params (ActionValue :type Boolean) (ElapsedSeconds :type "Float (double-precision)") (TriggeredSeconds :type "Float (double-precision)") (InputAction :type "InputAction Object Reference" :default "/Game/Input/IA_Punch.IA_Punch"))
  (:`Started`
    (if (not (`NavMovementComponent.IsFalling` (`Pawn.GetMovementComponent` (`GameplayStatics.GetPlayerCharacter` 0))))
      (`|PlayMontage` (`Character.Mesh` (`GameplayStatics.GetPlayerCharacter` 0)) "/Game/Anim/MN_Punch.MN_Punch"
        (:`then`
          (`self.StopMovement`)
          (`CharacterMovementComponent.DisableMovement` (`Character.CharacterMovement` (`GameplayStatics.GetPlayerCharacter` 0))))
        (:`OnCompleted`
          (`CharacterMovementComponent.SetMovementMode` (`Character.CharacterMovement` (`GameplayStatics.GetPlayerCharacter` 0)) "MOVE_Walking" 0 :!label _label)))))
  (:`Completed`
    (goto _label)))

(fn `UserConstructionScript`)