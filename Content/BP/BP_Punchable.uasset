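; BP_Punchable is an actor the player can knock away to damage the boss.
; PunchPunchable applies an impulse to its Sphere, pointing away from the player character and scaled by distance, using only X and Y, then destroys the actor after a delay.
; Overlapping BP_Boss prints a debug string, calls the boss's LifeLoss and destroys the actor immediately.
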(event Custom|PunchPunchable
  (bind _asbp_chara (Utilities|Casting|CastToBP_Chara (Game|GetPlayerCharacter 0)))
  (|CollapseGraph_2 (Variables|Default|GetSphere) (* (- (Transformation|GetWorldLocation (Variables|Default|GetSphere)) (Transformation|GetWorldLocation (Variables|/Script/Engine.Actor|GetRootComponent _asbp_chara))) 2e+03))
  (Utilities|FlowControl|Delay 3.0)
  (Actor|DestroyActor))

(event Collision|EventActorBeginOverlap
  (params (OtherActor :type Actor%20Object%20Reference))
  (bind _asbp_boss (Utilities|Casting|CastToBP_Boss OtherActor))
  (Development|PrintString "Hello")
  (Default|LifeLoss _asbp_boss)
  (Actor|DestroyActor))

(fn ConstructionScript)