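; Component that traces from the player's view direction to trigger grab or pull interactions on the actor it hits.
; Trace casts a thin box trace from slightly above player character zero along control rotation, with persistent debug drawing and printed hit distance.
; Hit I_Enemies actors receive GRABBEDMessage only beyond a distance threshold; otherwise, non-enemy I_Outlet actors receive PulledMessage.
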(event `Trace`
  (bind _returnvalue (`GameplayStatics.GetPlayerCharacter` 0))
  (bind _x (.x (`Actor.K2_GetActorLocation` _returnvalue)))
  (bind _y (.y (`Actor.K2_GetActorLocation` _returnvalue)))
  (bind _returnvalue_2 (+ (.z (`Actor.K2_GetActorLocation` _returnvalue)) 50.0))
  (bind (_returnvalue_x _returnvalue_y _returnvalue_z) (`KismetMathLibrary.BreakVector` (* (`KismetMathLibrary.GetForwardVector` (`Pawn.GetControlRotation` _returnvalue)) 3000.0)))
  (bind _outhit (`KismetSystemLibrary.BoxTraceSingle` :`Start` (`KismetMathLibrary.MakeVector` _x _y _returnvalue_2) :`End` (`KismetMathLibrary.MakeVector` (+ _x _returnvalue_x) (+ _y _returnvalue_y) (+ _returnvalue_2 _returnvalue_z)) :`HalfSize` (3.0 3.0 3.0) :`TraceChannel` "TraceTypeQuery1" :`DrawDebugType` "Persistent"))
  (bind (_bblockinghit _binitialoverlap _time _distance _location _impactpoint _normal _impactnormal _physmat _hitactor) (`GameplayStatics.BreakHitResult` _outhit))
  (`KismetSystemLibrary.PrintString` (`KismetStringLibrary.Conv_DoubleToString` _distance))
  (if (`KismetSystemLibrary.DoesImplementInterface` _hitactor "/Game/BP/Interface/I_Enemies.I_Enemies_C")
    (if (> _distance 2200.0)
      (message `/Game/BP/Interface/I_Enemies.GRABBED` _hitactor))
    (elif (`KismetSystemLibrary.DoesImplementInterface` _hitactor "/Game/BP/Interface/I_Outlet.I_Outlet_C")
      (message `/Game/BP/Interface/I_Outlet.Pulled` _hitactor))))