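; BP_SpawnerMov is a moving spawner that keeps supplying BP_Punchable actors.
; Its construction script gives InterpToMovement two relative control points from BeginLocation and EndLocation, timed by Duration.
; On BeginPlay it spawns a punchable slightly above its StaticMesh.
; When a punchable ends overlap with the spawner, it waits through a fixed delay and spawns another at the mesh's current position.
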(event `self.ReceiveBeginPlay`
  (`|SpawnActorFromClass` "/Game/BP/BP_Punchable.BP_Punchable_C" (`KismetMathLibrary.MakeTransform` (+ (`SceneComponent.K2_GetComponentLocation` (`self.StaticMesh`)) (0.0 0.0 30.0))) "Undefined" "OverrideRootScale" null null :!label _label))

(event `self.ReceiveActorEndOverlap`
  (params (OtherActor :type "Actor Object Reference"))
  (cast `/Game/BP/BP_Punchable` OtherActor)
  (`KismetSystemLibrary.Delay` 5.0)
  (goto _label))

(fn `UserConstructionScript`
  (bind _interptomovement (`self.InterpToMovement`))
  (set `InterpToMovementComponent.ControlPoints` (`|MakeArray` (make `InterpControlPoint` (`self.BeginLocation`)) (make `InterpControlPoint` (`self.EndLocation`))) _interptomovement)
  (set `InterpToMovementComponent.Duration` (`self.Duation`) _interptomovement))