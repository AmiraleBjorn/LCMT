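; BP_EnnemisBlock is a destructible enemy block that rewards the player when destroyed.
; Each HealthLoss event decrements its Health by one and destroys the actor when that reaches zero.
; On destruction it casts the player character to BP_Chara and adds a fixed amount to its NotHealth value, capped at one.
; The file does not call HealthLoss itself, and its construction script is empty.
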(event `HealthLoss`
  (bind _result (`/Engine/EditorBlueprintResources/StandardMacros.DecrementInt` (`self.Health`))
    (:`  `
      (bind _output_get (set `self.Health` _result))
      (if (== _output_get 0)
        (`self.K2_DestroyActor`)
        (bind _asbp_chara (cast `/Game/BP/BP_Chara` (`GameplayStatics.GetPlayerCharacter` 0)))
        (bind _output_get_2 (set `/Game/BP/BP_Chara.NotHealth` (+ (`/Game/BP/BP_Chara.NotHealth` _asbp_chara) 0.5) _asbp_chara))
        (if (> _output_get_2 1.0)
          (set `/Game/BP/BP_Chara.NotHealth` 1.0 _asbp_chara))))))

(fn `UserConstructionScript`)