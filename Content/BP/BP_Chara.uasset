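; Player character Blueprint with whip, roar, dash and pull abilities, plus a draining NotHealth value that opens the GameOver level below zero.
; NotHealth falls every tick, and each roar costs extra.
; Game-time cooldowns gate the whip, which fires the ACLineTrace component, and the roar, which invokes CallRoar.
; Dash and Pull pair an upward LaunchCharacter with a launch along controller facing or toward the given Outlet, respectively.
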(event `Pull`
  (params (Outlet :type "/Game/BP/BP_Outlet Object Reference"))
  (`self.LaunchCharacter` (0.0 0.0 200.0))
  (`self.LaunchCharacter` (* (- (`SceneComponent.K2_GetComponentLocation` (`Actor.RootComponent` Outlet)) (`SceneComponent.K2_GetComponentLocation` (`self.CapsuleComponent`))) 2.0)))

(event `self.ReceiveTick`
  (params (DeltaSeconds :type "Float (single-precision)"))
  (`/Engine/EditorBlueprintResources/StandardMacros.IsValid` self
    (:`Is Valid`
      (bind _output_get (set `self.NotHealth` (- (`self.NotHealth`) 0.001)))
      (if (< _output_get 0.0)
        (`GameplayStatics.OpenLevelBySoftObjectPtr` "/Game/Map/GameOver.GameOver")))))

(event `Rallonge`
  (bind _returnvalue (`KismetSystemLibrary.GetGameTimeInSeconds`))
  (`/Engine/EditorBlueprintResources/StandardMacros.CompareFloat` (`self.Whip CD`) (`KismetSystemLibrary.GetGameTimeInSeconds`)
    (:`<`
      (set `self.Whip CD` 0.0)
      (`/Game/BP/Componnent/AC_LineTrace.Trace` (`self.AC_LineTrace`))
      (set `self.GameTimeCDWhip` _returnvalue)
      (set `self.Whip CD` (+ _returnvalue 1.0)))))

(event `Roared`
  (bind _returnvalue (`KismetSystemLibrary.GetGameTimeInSeconds`))
  (`/Engine/EditorBlueprintResources/StandardMacros.CompareFloat` (`self.Roar CD`) (`KismetSystemLibrary.GetGameTimeInSeconds`)
    (:`<`
      (set `self.Roar CD` 0.0)
      (`self.Roar`)
      (set `self.GameTimeCDRoar` _returnvalue)
      (set `self.Roar CD` (+ _returnvalue 10.0))
      (set `self.NotHealth` (- (`self.NotHealth`) 0.1)))))

(event `Dash`
  (bind (_returnvalue_roll _returnvalue_pitch _returnvalue_yaw) (`KismetMathLibrary.BreakRotator` (`SceneComponent.K2_GetComponentRotation` (`Actor.RootComponent` (`GameplayStatics.GetPlayerController` 0)))))
  (`self.LaunchCharacter` self (0.0 0.0 1000.0) false false)
  (`self.LaunchCharacter` (* (`KismetMathLibrary.GetForwardVector` (`KismetMathLibrary.MakeRotator` 0.0 _returnvalue_pitch _returnvalue_yaw)) 2000.0)))

(fn `UserConstructionScript`)