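; BP_IA_Roam is an AI character that wanders and can be pulled toward the player.
; From BeginPlay it moves to a random reachable point within a fixed radius of itself, picking a new one only when a move succeeds.
; The GRABBED event gives a small upward launch, then after a brief delay launches it toward the BP_Chara player with velocity scaled by their separation.
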(event `self.ReceiveBeginPlay`
  (`self.Roam`))

(event `Roam`
  (`|AIMoveTo` self (`NavigationSystemV1.K2_GetRandomReachablePointInRadius` (`self.K2_GetActorLocation`) 2500.0 null null) null
    (:`OnSuccess`
      (`self.Roam`))))

(event `/Game/BP/Interface/I_Enemies.GRABBED`
  (bind _asbp_chara (cast `/Game/BP/BP_Chara` (`GameplayStatics.GetPlayerCharacter` 0)))
  (`self.LaunchCharacter` (0.0 0.0 200.0))
  (`KismetSystemLibrary.Delay` 0.01)
  (`self.LaunchCharacter` (* (- (`SceneComponent.K2_GetComponentLocation` (`Actor.RootComponent` _asbp_chara)) (`SceneComponent.K2_GetComponentLocation` (`self.CapsuleComponent`))) 5.0)))

(fn `UserConstructionScript`)