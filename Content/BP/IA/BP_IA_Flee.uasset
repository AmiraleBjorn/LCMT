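; BP_IA_Flee is an AI character that runs away from the player and can be pulled toward them when grabbed.
; From BeginPlay, RunAway repeatedly issues a short AIMoveTo directly away from BP_Chara at its own height, restarting on success or failure.
; GRABBED launches it upward, then after a tiny delay launches it toward the player with velocity proportional to their separation.
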(event `self.ReceiveBeginPlay`
  (bind _asbp_chara (cast `/Game/BP/BP_Chara` (`GameplayStatics.GetPlayerCharacter` 0)))
  (set `self.Player_Ref` _asbp_chara)
  (`self.RunAway`))

(event `RunAway`
  (bind _returnvalue (`self.K2_GetActorLocation`))
  (`|AIMoveTo` self (`KismetMathLibrary.MakeVector` (.x (+ _returnvalue (* (`KismetMathLibrary.GetForwardVector` (`KismetMathLibrary.FindLookAtRotation` _returnvalue (`self.K2_GetActorLocation` (`self.Player_Ref`)))) -50.0))) (.y (+ _returnvalue (* (`KismetMathLibrary.GetForwardVector` (`KismetMathLibrary.FindLookAtRotation` _returnvalue (`self.K2_GetActorLocation` (`self.Player_Ref`)))) -50.0))) (.z _returnvalue)) null
    (:`OnSuccess`
      _)
    (:`OnFail`
      _))
  (`self.RunAway`))

(event `/Game/BP/Interface/I_Enemies.GRABBED`
  (bind _asbp_chara (cast `/Game/BP/BP_Chara` (`GameplayStatics.GetPlayerCharacter` 0)))
  (`self.LaunchCharacter` (0.0 0.0 200.0))
  (`KismetSystemLibrary.Delay` 0.01)
  (`self.LaunchCharacter` (* (- (`SceneComponent.K2_GetComponentLocation` (`Actor.RootComponent` _asbp_chara)) (`SceneComponent.K2_GetComponentLocation` (`self.CapsuleComponent`))) 5.0)))

(fn `UserConstructionScript`)