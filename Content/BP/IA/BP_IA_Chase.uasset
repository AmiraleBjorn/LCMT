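; BP_IA_Chase is an AI character that chases the player on sight and wanders otherwise.
; PawnSensing starts an AIMoveTo on BP_Chara, with a retriggerable delay clearing the seen flag once sightings stop.
; Tick drops the chase after a short grace delay, then issues moves to random reachable points at random intervals.
; GRABBED pops the character upward, then launches it toward the player with velocity scaled by distance.
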(event `/Game/BP/Interface/I_Enemies.GRABBED`
  (bind _asbp_chara (cast `/Game/BP/BP_Chara` (`GameplayStatics.GetPlayerCharacter` 0)))
  (`self.LaunchCharacter` (0.0 0.0 200.0))
  (`KismetSystemLibrary.Delay` 0.01)
  (`self.LaunchCharacter` (* (- (`SceneComponent.K2_GetComponentLocation` (`Actor.RootComponent` _asbp_chara)) (`SceneComponent.K2_GetComponentLocation` (`self.CapsuleComponent`))) 5.0)))

(event `self.PawnSensing.OnSeePawn`
  (params (Pawn :type "Pawn Object Reference"))
  (bind _asbp_chara (cast `/Game/BP/BP_Chara` Pawn))
  (`|ExecutionSequence`
    (:`then_0`
      (set `self.See_Player` true)
      (set `self.IsChasing?` true)
      (`|AIMoveTo` self (0.0 0.0 0.0) _asbp_chara))
    (:`then_1`
      (`KismetSystemLibrary.RetriggerableDelay` 0.6)
      (set `self.See_Player` false))))

(event `self.ReceiveTick`
  (params (DeltaSeconds :type "Float (single-precision)"))
  (bind _see_player (`self.See_Player`))
  (`|ExecutionSequence`
    (:`then_0`
      (if (not _see_player)
        (`KismetSystemLibrary.Delay` 0.4)
        (if (not _see_player)
          (set `self.IsChasing?` false))))
    (:`then_1`
      (if (not (`self.IsChasing?`))
        (`KismetSystemLibrary.Delay` (`KismetMathLibrary.RandomFloatInRange` 2.0 5.0))
        (`|AIMoveTo` self (`NavigationSystemV1.K2_GetRandomReachablePointInRadius` (`self.K2_GetActorLocation`) 2500.0 null null) null)))))

(fn `UserConstructionScript`)