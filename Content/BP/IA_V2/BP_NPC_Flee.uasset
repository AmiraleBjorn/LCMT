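; Fleeing NPC character that the player can scare with a roar, punch or grab.
; The player's roar halts it for two seconds, behind a distance check that compares its own root and capsule.
; Punches cost health and launch it up then away; death sets the player's NotHealth to full.
; Grabs launch it toward the player, and pawn sensing sets HasSeenPlayer on its AI blackboard.
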(event `self.ReceiveBeginPlay`
  (bind _asbp_chara (cast `/Game/BP/BP_Chara` (`GameplayStatics.GetPlayerCharacter` 0)))
  (add `/Game/BP/BP_Chara.Roar` _asbp_chara (delegate `Terrified`)))

(event `Terrified`
  (bind _charactermovement (`self.CharacterMovement`))
  (if (< (`KismetMathLibrary.VSize` (- (`SceneComponent.K2_GetComponentLocation` (`self.RootComponent`)) (`SceneComponent.K2_GetComponentLocation` (`self.CapsuleComponent`)))) 1000.0)
    (set `CharacterMovementComponent.MaxWalkSpeed` 0.0 _charactermovement)
    (`KismetSystemLibrary.Delay` 2.0)
    (set `CharacterMovementComponent.MaxWalkSpeed` 350.0 _charactermovement)))

(event `PunchedFlee`
  (bind _result (`/Engine/EditorBlueprintResources/StandardMacros.DecrementInt` (`self.NPCHealth`))
    (:`  `
      (set `self.NPCHealth` _result)
      (bind _asgi_main (cast `/Game/Game/GI_Main` (`GameplayStatics.GetGameInstance`)))
      (`GameplayStatics.PlaySound2D` "/Game/Sound_design/Ennemy-kill.Ennemy-kill" (`/Game/Game/GI_Main.VOLUME` _asgi_main) 1.0 0.0 null null)
      (if (== _result 0)
        (`self.K2_DestroyActor`)
        (bind _asbp_chara (cast `/Game/BP/BP_Chara` (`GameplayStatics.GetPlayerCharacter` 0)))
        (if true
          (set `/Game/BP/BP_Chara.NotHealth` 1.0 _asbp_chara)
          (else
            (set `/Game/BP/BP_Chara.NotHealth` (+ (`/Game/BP/BP_Chara.NotHealth` _asbp_chara) 0.1) _asbp_chara)))
        (else
          (bind _asbp_chara_2 (cast `/Game/BP/BP_Chara` (`GameplayStatics.GetPlayerCharacter` 0)))
          (`self.LaunchCharacter` (0.0 0.0 200.0))
          (`KismetSystemLibrary.Delay` 0.01)
          (`self.LaunchCharacter` (* (- (`SceneComponent.K2_GetComponentLocation` (`self.CapsuleComponent`)) (`SceneComponent.K2_GetComponentLocation` (`Actor.RootComponent` _asbp_chara_2))) 5.0)))))))

(event `CustomEvent`
  (bind _asbp_chara (cast `/Game/BP/BP_Chara` (`GameplayStatics.GetPlayerCharacter` 0)))
  (`self.LaunchCharacter` (0.0 0.0 200.0))
  (`KismetSystemLibrary.Delay` 0.01)
  (`self.LaunchCharacter` (* (- (`SceneComponent.K2_GetComponentLocation` (`Actor.RootComponent` _asbp_chara)) (`SceneComponent.K2_GetComponentLocation` (`self.CapsuleComponent`))) 5.0)))

(event `/Game/BP/Interface/I_Enemies.GRABBED`
  (bind _asbp_chara (cast `/Game/BP/BP_Chara` (`GameplayStatics.GetPlayerCharacter` 0)))
  (`self.LaunchCharacter` (0.0 0.0 200.0))
  (`KismetSystemLibrary.Delay` 0.01)
  (`self.LaunchCharacter` (* (- (`SceneComponent.K2_GetComponentLocation` (`Actor.RootComponent` _asbp_chara)) (`SceneComponent.K2_GetComponentLocation` (`self.CapsuleComponent`))) 6.0)))

(event `self.PawnSensing.OnSeePawn`
  (params (Pawn :type "Pawn Object Reference"))
  (cast `/Game/BP/BP_Chara` Pawn)
  (`BlackboardComponent.SetValueAsBool` (`AIBlueprintHelperLibrary.GetBlackboard` (`AIBlueprintHelperLibrary.GetAIController` self)) "HasSeenPlayer" true))

(fn `UserConstructionScript`)