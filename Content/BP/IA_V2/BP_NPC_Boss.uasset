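; Boss NPC character that shoves the player on overlap, can be stunned, and takes punch damage.
; KnockedBack destroys the incoming Punchable, launches the boss and stuns it for two seconds, suspending its shove.
; PunchedBoss lowers health and plays a sound, then either knocks the boss away from the player or, once health drops to 1, destroys it and triggers HUD Cutscene4.
; Knockbacks use a small upward launch followed by a delayed directional one.
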(event OnComponentBeginOverlap(r)
  (params (OverlappedComponent :type Primitive%20Component%20Object%20Reference) (OtherActor :type Actor%20Object%20Reference) (OtherComp :type Primitive%20Component%20Object%20Reference) (OtherBodyIndex :type Integer) (bFromSweep :type Boolean) (SweepResult :type Hit%20Result%20Structure%20%28by%20ref%29))
  (if (not (Variables|Default|GetIsStuned))
    (bind _asbp_chara (Utilities|Casting|CastToBP_Chara OtherActor))
    (Default|PushedBack _asbp_chara self 3.0)))

(event Custom|PunchedBoss
  (Variables|Default|SetBossHealth (- (Variables|Default|GetBossHealth) 1))
  (bind _asgi_main (Utilities|Casting|CastToGI_Main (Game|GetGameInstance)))
  (Audio|PlaySound2D "/Game/Sound_design/Ennemy-kill.Ennemy-kill" (Variables|/Game/Game/GI_Main.GI_Main_C|GetVOLUME _asgi_main) 1.0 0.0 0 0)
  (if (== (- (Variables|Default|GetBossHealth) 1) 0)
    (Actor|DestroyActor)
    (bind _ashud_main (Utilities|Casting|CastToHUD_Main (HUD|GetHUD (Game|GetPlayerController 0))))
    (Default|Cutscene4 _ashud_main)
    (else
      (bind _asbp_chara (Utilities|Casting|CastToBP_Chara (Game|GetPlayerCharacter 0)))
      (|CollapseGraph_2_2)
      (Utilities|FlowControl|Delay 0.01)
      (|CollapseGraph_0_2_2 (* (- (Transformation|GetWorldLocation (Variables|Collision|GetCapsuleComponent)) (Transformation|GetWorldLocation (Variables|/Script/Engine.Actor|GetRootComponent _asbp_chara))) 5.0)))))

(event Custom|KnockedBack
  (params (Punchable :type BP%20Punchable%20Object%20Reference))
  (bind _rootcomponent (Variables|/Script/Engine.Actor|GetRootComponent Punchable))
  (bind _rootcomponent_2 (Variables|Transformation|GetRootComponent))
  (bind _capsulecomponent (Variables|Collision|GetCapsuleComponent))
  (bind _capsulecomponent_2 (Variables|Collision|GetCapsuleComponent))
  (bind _returnvalue (Transformation|GetWorldLocation _rootcomponent_2))
  (bind _returnvalue_2 (Transformation|GetWorldLocation _capsulecomponent))
  (bind _returnvalue_3 (Transformation|GetWorldLocation _rootcomponent))
  (bind _returnvalue_4 (Transformation|GetWorldLocation _capsulecomponent_2))
  (bind _returnvalue_5 (- _returnvalue_2 _returnvalue_3))
  (bind _returnvalue_6 (- _returnvalue_4 _returnvalue))
  (bind _returnvalue_7 (* _returnvalue_5 1e+04))
  (bind _returnvalue_8 (* _returnvalue_6 1e+04))
  (|CollapseGraph_2)
  (Utilities|FlowControl|Delay 0.01)
  (|CollapseGraph_0_2 (Math|Vector|MakeVector (.x _returnvalue_7) (.y _returnvalue_7) 0.0) 0.0 0.0 0.0)
  (Actor|DestroyActor Punchable)
  (Variables|Default|SetIsStuned true)
  (Utilities|FlowControl|Delay 2.0)
  (Variables|Default|SetIsStuned false)
  (|CollapseGraph_2_3)
  (Utilities|FlowControl|Delay 0.01)
  (|CollapseGraph_0_2_3 (Math|Vector|MakeVector (.x _returnvalue_8) (.y _returnvalue_8) 0.0) 0.0 0.0 0.0))

(fn ConstructionScript)