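; NPC character that reacts to the player BP_Chara's roar and punches.
; On the Roar event it freezes for three seconds, though the range check compares its own root and capsule, so it likely always passes.
; Each punch decrements health and launches it upward, then away from the player after a brief delay.
; At zero health it destroys itself and increases the player's NotHealth.
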(event `self.ReceiveBeginPlay`
  (bind _asbp_chara (cast `/Game/BP/BP_Chara` (`GameplayStatics.GetPlayerCharacter` 0)))
  (add `/Game/BP/BP_Chara.Roar` _asbp_chara (delegate `Terrified`)))

(event `Terrified`
  (bind _charactermovement (`self.CharacterMovement`))
  (if (< (`KismetMathLibrary.VSize` (- (`SceneComponent.K2_GetComponentLocation` (`self.RootComponent`)) (`SceneComponent.K2_GetComponentLocation` (`self.CapsuleComponent`)))) 1000.0)
    (set `CharacterMovementComponent.MaxWalkSpeed` 0.0 _charactermovement)
    (`KismetSystemLibrary.Delay` 3.0)
    (set `CharacterMovementComponent.MaxWalkSpeed` 350.0 _charactermovement)))

(event `Punched`
  (bind _npchealth (`self.NPCHealth`))
  (bind _result (`/Engine/EditorBlueprintResources/StandardMacros.DecrementInt` _npchealth)
    (:`  `
      (set `self.NPCHealth` _result)
      (if (== _npchealth 0)
        (`self.K2_DestroyActor`)
        (bind _asbp_chara (cast `/Game/BP/BP_Chara` (`GameplayStatics.GetPlayerCharacter` 0)))
        (set `/Game/BP/BP_Chara.NotHealth` (+ (`/Game/BP/BP_Chara.NotHealth` _asbp_chara) 0.1) _asbp_chara)
        (else
          (bind _asbp_chara_2 (cast `/Game/BP/BP_Chara` (`GameplayStatics.GetPlayerCharacter` 0)))
          (`self.LaunchCharacter` (0.0 0.0 200.0))
          (`KismetSystemLibrary.Delay` 0.01)
          (`self.LaunchCharacter` (* (- (`SceneComponent.K2_GetComponentLocation` (`self.CapsuleComponent`)) (`SceneComponent.K2_GetComponentLocation` (`Actor.RootComponent` _asbp_chara_2))) 5.0)))))))

(fn `UserConstructionScript`)